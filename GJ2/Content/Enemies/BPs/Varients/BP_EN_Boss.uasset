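; Boss enemy pawn that chases, faces, shoots and contact-damages the player, then spawns a level transition on death if a level is named.
; When the player is in range, Tick drives all behavior and scales health and shield once, by 25% per kill from Globals.
; Randomly timed phases either aim or spin the arrow pivot and set the fire interval, with kill count widening the pool of available attack patterns.
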(event Custom|Face%20Player
  (params (Delta%20Time :type Float%20%28single-precision%29))
  (Utilities|IsValid (Game|GetPlayerCharacter 0)
    (:Is%20Valid
      (Transformation|SetWorldRotation (Variables|Default|GetCapsule) (Math|Interpolation|RInterpTo (Transformation|GetWorldRotation (Variables|Default|GetCapsule)) (Math|Rotator|MakeRotator 0.0 0.0 (.yaw (Math|Rotator|FindLookatRotation (Transformation|GetActorLocation) (Transformation|GetActorLocation (Game|GetPlayerCharacter 0))))) Delta%20Time 1e+01) false false))))

(event Custom|Move
  (Utilities|IsValid (Game|GetPlayerCharacter 0)
    (:Is%20Valid
      (if (> (Math|Vector|Distance(Vector) (Transformation|GetActorLocation) (Transformation|GetActorLocation (Game|GetPlayerCharacter 0))) (Variables|Default|GetTarget%20Range%20From%20Player))
        (Class|PawnMovementComponent|AddInputVector (Variables|Default|GetFloatingPawnMovement) (Math|Vector|GetForwardVector (Variables|Default|GetCapsule)) false)))))

(event Custom|Phase_2
  (Transformation|AddWorldRotation (Variables|Default|GetArrowPivot) "0,-2.000000, 0" false false)
  (Variables|Default|SetFire%20Interval 0.05))

(event Custom|On%20Death
  (CallFunction|StartNextLevel))

(event Custom|Phase_3
  (Transformation|AddWorldRotation (Variables|Default|GetArrowPivot) "0,45.000000, 0" false false)
  (Variables|Default|SetFire%20Interval 0.025))

(event Custom|Start%20Next%20Level
  (bind _level_to_open_on_death_name (Variables|Default|GetLevel%20To%20Open%20On%20Death%20Name))
  (if (Utilities|Name|NotEqual(Name) _level_to_open_on_death_name "None")
    (Game|SpawnActorfromClass "/Game/BPs/LevelTransition/BP_Level_Transition.BP_Level_Transition_C" (Transformation|GetActorTransform) "Undefined" 0 _level_to_open_on_death_name 1.0 0)))

(event Custom|Phase_0
  (bind _returnvalue (Game|GetPlayerCharacter 0))
  (Utilities|IsValid _returnvalue
    (:Is%20Valid
      (Transformation|SetWorldRotation (Variables|Default|GetArrowPivot) (Math|Rotator|FindLookatRotation (Transformation|GetWorldLocation (Variables|Default|GetArrowPivot)) (Transformation|GetActorLocation _returnvalue)) false false)
      (Variables|Default|SetFire%20Interval 1.0))))

(event Custom|Damage%20Player
  (bind _returnvalue (Game|GetPlayerCharacter 0))
  (Utilities|IsValid _returnvalue
    (:Is%20Valid
      (bind _asthird_person_character (Utilities|Casting|CastToThirdPersonCharacter _returnvalue))
      (if (< (Math|Vector|Distance(Vector) (Transformation|GetActorLocation) (Transformation|GetActorLocation (Game|GetPlayerCharacter 0))) (Variables|Default|GetDamage%20Distance))
        (bind _triggered (Default|BeginIframes _asthird_person_character))
        (if _triggered
          (Default|KnockbackPlayer _asthird_person_character (* (Math|Vector|GetForwardVector (Variables|Default|GetCapsule)) (Variables|Default|GetKnockback%20Force)))
          (Default|Damage (Variables|/Game/ThirdPersonBP/Blueprints/ThirdPersonCharacter.ThirdPersonCharacter_C|GetBP_HealthComponent _asthird_person_character) (Variables|Default|GetDamage%20Amount))
          (Audio|PlaySoundatLocation "/Game/Audio/Damage_Taken_Cue.Damage_Taken_Cue" (Transformation|GetActorLocation) "0, 0, 0" 1.0 1.0 0.0 0 0 0))))))

(event Custom|FireProjectile
  (bind _arrow (Variables|Default|GetArrow))
  (if (Variables|Default|GetcanFire)
    (Utilities|IsValid (Game|GetPlayerCharacter 0)
      (:Is%20Valid
        (if (<= (Math|Vector|Distance(Vector) (Transformation|GetActorLocation) (Transformation|GetActorLocation (Game|GetPlayerCharacter 0))) (Variables|Default|GetFire%20Range))
          (Game|SpawnActorfromClass "/Game/Enemies/BPs/Varients/BP_enemy_projectile.BP_enemy_projectile_C" (Math|Transform|MakeTransform (Transformation|GetWorldLocation _arrow) (Transformation|GetWorldRotation _arrow) "0.750000,0.750000,0.750000") "Undefined" 0 0)
          (Audio|PlaySoundatLocation "/Game/Audio/EnemyFire_Cue.EnemyFire_Cue" (Transformation|GetActorLocation) "0, 0, 0" 1.5 1.0 0.05 0 0 0)
          (Variables|Default|SetcanFire false)
          (Utilities|FlowControl|Delay (Variables|Default|GetFire%20Interval))
          (Variables|Default|SetcanFire true))))))

(event Custom|PhaseChange
  (Utilities|FlowControl|Delay (Math|Random|RandomFloatinRange 2.0 4.0))
  (bind _asglobals (Utilities|Casting|CastToGlobals (Game|GetGameInstance)))
  (Utilities|FlowControl|ForLoopwithBreak 0 2 :!label _label
    (:LoopBody
      (if (!= (Variables|Default|GetPhase) (Math|Random|RandomIntegerinRange 0 (Math|Integer|Clamp(Integer) (Math|Float|Round (* (Variables|/Game/ThirdPersonBP/Blueprints/Globals.Globals_C|GetKillCount _asglobals) (/ (Math|Conversions|ToFloat(Integer) (Variables|Default|GetAttack%20Max%20Count)) (Math|Conversions|ToFloat(Integer) (Variables|Default|GetKills%20needed%20for%20all%20attacks%20unlocked))))) 0 (Variables|Default|GetAttack%20Max%20Count))))
        (goto _label Break)))
    (:Completed
      (Variables|Default|SetPhase (Math|Random|RandomIntegerinRange 0 (Math|Integer|Clamp(Integer) (Math|Float|Round (* (Variables|/Game/ThirdPersonBP/Blueprints/Globals.Globals_C|GetKillCount _asglobals) (/ (Math|Conversions|ToFloat(Integer) (Variables|Default|GetAttack%20Max%20Count)) (Math|Conversions|ToFloat(Integer) (Variables|Default|GetKills%20needed%20for%20all%20attacks%20unlocked))))) 0 (Variables|Default|GetAttack%20Max%20Count)))))))

(event Custom|Phases_Switch
  (switch int (Variables|Default|GetPhase)
    (:0
      (CallFunction|Phase0))
    (:1
      (CallFunction|Phase1))
    (:2
      (CallFunction|Phase2))
    (:3
      (CallFunction|Phase3))
    (:4
      (CallFunction|Phase4))
    (:5
      (CallFunction|Phase5))))

(event Custom|Phase_5
  (bind _returnvalue (Game|GetPlayerCharacter 0))
  (Utilities|IsValid _returnvalue
    (:Is%20Valid
      (Transformation|SetWorldRotation (Variables|Default|GetArrowPivot) (Math|Rotator|FindLookatRotation (Transformation|GetWorldLocation (Variables|Default|GetArrowPivot)) (Transformation|GetActorLocation _returnvalue)) false false)
      (Variables|Default|SetFire%20Interval 0.5))))

(event Custom|Phase_4
  (Transformation|AddWorldRotation (Variables|Default|GetArrowPivot) "0,90.000000, 0" false false)
  (Variables|Default|SetFire%20Interval 0.025))

(event Custom|Phase_1
  (Transformation|AddWorldRotation (Variables|Default|GetArrowPivot) "0,2.000000, 0" false false)
  (Variables|Default|SetFire%20Interval 0.05))

(event Custom|Scale%20Vitality
  (bind _bp_healthcomponent (Variables|Default|GetBP_HealthComponent))
  ;[1 0.1658 0.3875] Scale Vitality by +25% Per Kill
  (Utilities|FlowControl|DoOnce false
    (:Completed
      (bind _scaled_amount (CallFunction|AdditiveScalePerKill (Variables|/Game/BPs/Components/BP_HealthComponent.BP_HealthComponent_C|GetHP%20Max _bp_healthcomponent) 0.25))
      (Variables|/Game/BPs/Components/BP_HealthComponent.BP_HealthComponent_C|SetHP%20Max _bp_healthcomponent _scaled_amount)
      (bind _scaled_amount_2 (CallFunction|AdditiveScalePerKill (Variables|/Game/BPs/Components/BP_HealthComponent.BP_HealthComponent_C|GetShield%20Max _bp_healthcomponent) 0.25))
      (Variables|/Game/BPs/Components/BP_HealthComponent.BP_HealthComponent_C|SetShield%20Max _bp_healthcomponent _scaled_amount_2)
      (bind _scaled_amount_3 (CallFunction|AdditiveScalePerKill (Variables|/Game/BPs/Components/BP_HealthComponent.BP_HealthComponent_C|GetHP%20Amount _bp_healthcomponent) 0.25))
      (Variables|/Game/BPs/Components/BP_HealthComponent.BP_HealthComponent_C|SetHP%20Amount _bp_healthcomponent _scaled_amount_3)
      (bind _scaled_amount_4 (CallFunction|AdditiveScalePerKill (Variables|/Game/BPs/Components/BP_HealthComponent.BP_HealthComponent_C|GetShield%20Amount _bp_healthcomponent) 0.25))
      (Variables|/Game/BPs/Components/BP_HealthComponent.BP_HealthComponent_C|SetShield%20Amount _bp_healthcomponent _scaled_amount_4))))

(event EventBeginPlay
  (|CallParentFunction)
  (EventDispatchers|BindEventtoOnDeath (Variables|Default|GetBP_HealthComponent) (delegate Custom|On%20Death)))

(event Collision|EventActorBeginOverlap
  (params (OtherActor :type Actor%20Object%20Reference)))

(event EventTick
  (params (DeltaSeconds :type Float%20%28single-precision%29))
  (|CallParentFunction DeltaSeconds)
  (bind _isplayerinrange (CallFunction|IsPlayerinRange))
  (if _isplayerinrange
    (CallFunction|ScaleVitality)
    (CallFunction|FacePlayer DeltaSeconds)
    (CallFunction|Move)
    (CallFunction|DamagePlayer)
    (CallFunction|FireProjectile)
    (CallFunction|PhaseChange)
    (CallFunction|PhasesSwitch)))

(fn ConstructionScript
  (|CallParentFunction))

(fn AdditiveScalePerKill
  (params (Input%20Amount :type Float%20%28single-precision%29) (Additive%20Scale%20Amount :type Float%20%28single-precision%29))
  (bind _asglobals (Utilities|Casting|CastToGlobals (Game|GetGameInstance)))
  (return (+ Input%20Amount (* (* (Variables|/Game/ThirdPersonBP/Blueprints/Globals.Globals_C|GetKillCount _asglobals) Additive%20Scale%20Amount) Input%20Amount))))