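; Ranged enemy variant that chases the player, fires projectiles and deals knockback damage up close.
; While the player is in range, Tick yaws the capsule toward them, moves forward until a target distance, and fires from an Arrow on a Delay-gated cooldown.
; Close hits apply knockback and damage only when the player's BeginIframes succeeds.
; Health component damage events refresh the health and shield values on its widget.
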(event OnDamageRecieved(BP_HealthComponent)
  (bind _bp_healthcomponent (Variables|Default|GetBP_HealthComponent))
  (bind _enemyhealth_ui (Variables|Default|GetEnemyHealth_UI))
  ;[1 1 1] Decreases health bar widget
  (Variables|/Game/UI/EnemyHealth_UI.EnemyHealth_UI_C|SetHealth _enemyhealth_ui (Variables|/Game/BPs/Components/BP_HealthComponent.BP_HealthComponent_C|GetHP%20Amount _bp_healthcomponent))
  ;[1 1 1] Same but for shield
  (Variables|/Game/UI/EnemyHealth_UI.EnemyHealth_UI_C|SetShield _enemyhealth_ui (Variables|/Game/BPs/Components/BP_HealthComponent.BP_HealthComponent_C|GetShield%20Amount _bp_healthcomponent)))

(event Custom|Face%20Player
  (params (Delta%20Time :type Float%20%28single-precision%29))
  (Utilities|IsValid (Game|GetPlayerCharacter 0)
    (:Is%20Valid
      (Transformation|SetWorldRotation (Variables|Default|GetCapsule) (Math|Interpolation|RInterpTo (Transformation|GetWorldRotation (Variables|Default|GetCapsule)) (Math|Rotator|MakeRotator 0.0 0.0 (.yaw (Math|Rotator|FindLookatRotation (Transformation|GetActorLocation) (Transformation|GetActorLocation (Game|GetPlayerCharacter 0))))) Delta%20Time 1e+01) false false))))

(event Custom|Move
  (Utilities|IsValid (Game|GetPlayerCharacter 0)
    (:Is%20Valid
      (if (> (Math|Vector|Distance(Vector) (Transformation|GetActorLocation) (Transformation|GetActorLocation (Game|GetPlayerCharacter 0))) (Variables|Default|GetTarget%20Range%20From%20Player))
        (Class|PawnMovementComponent|AddInputVector (Variables|Default|GetFloatingPawnMovement) (Math|Vector|GetForwardVector (Variables|Default|GetCapsule)) false)))))

(event Custom|Damage%20Player
  (bind _returnvalue (Game|GetPlayerCharacter 0))
  (Utilities|IsValid _returnvalue
    (:Is%20Valid
      (bind _asthird_person_character (Utilities|Casting|CastToThirdPersonCharacter _returnvalue))
      (if (< (Math|Vector|Distance(Vector) (Transformation|GetActorLocation) (Transformation|GetActorLocation (Game|GetPlayerCharacter 0))) (Variables|Default|GetDamage%20Distance))
        (bind _triggered (Default|BeginIframes _asthird_person_character))
        (if _triggered
          (Default|KnockbackPlayer _asthird_person_character (* (Math|Vector|GetForwardVector (Variables|Default|GetCapsule)) (Variables|Default|GetKnockback%20Force)))
          (Default|Damage (Variables|/Game/ThirdPersonBP/Blueprints/ThirdPersonCharacter.ThirdPersonCharacter_C|GetBP_HealthComponent _asthird_person_character) (Variables|Default|GetDamage%20Amount)))))))

(event Custom|FireProjectile
  (bind _arrow (Variables|Default|GetArrow))
  (if (Variables|Default|GetcanFire)
    (Utilities|IsValid (Game|GetPlayerCharacter 0)
      (:Is%20Valid
        (if (<= (Math|Vector|Distance(Vector) (Transformation|GetActorLocation) (Transformation|GetActorLocation (Game|GetPlayerCharacter 0))) (Variables|Default|GetFire%20Range))
          (Game|SpawnActorfromClass "/Game/Enemies/BPs/Varients/BP_enemy_projectile.BP_enemy_projectile_C" (Math|Transform|MakeTransform (Transformation|GetWorldLocation _arrow) (Transformation|GetWorldRotation _arrow) "1,1,1") "Undefined" 0 0)
          (Variables|Default|SetcanFire false)
          (Utilities|FlowControl|Delay (Variables|Default|GetFire%20Interval))
          (Variables|Default|SetcanFire true))))))

(event EventBeginPlay
  (bind _bp_healthcomponent (Variables|Default|GetBP_HealthComponent))
  (|CallParentFunction)
  ;[1 1 1] Sets up the health bar widget
  (bind _asenemy_health_ui (Utilities|Casting|CastToEnemyHealth_UI (UserInterface|GetUserWidgetObject (Variables|Default|GetWidget))))
  (bind _output_get (Variables|Default|SetEnemyHealth_UI _asenemy_health_ui))
  (Variables|/Game/UI/EnemyHealth_UI.EnemyHealth_UI_C|SetHealth _output_get (Variables|/Game/BPs/Components/BP_HealthComponent.BP_HealthComponent_C|GetHP%20Amount _bp_healthcomponent))
  (Variables|/Game/UI/EnemyHealth_UI.EnemyHealth_UI_C|SetShield _output_get (Variables|/Game/BPs/Components/BP_HealthComponent.BP_HealthComponent_C|GetShield%20Amount _bp_healthcomponent)))

(event Collision|EventActorBeginOverlap
  (params (OtherActor :type Actor%20Object%20Reference)))

(event EventTick
  (params (DeltaSeconds :type Float%20%28single-precision%29))
  (|CallParentFunction DeltaSeconds)
  (bind _isplayerinrange (CallFunction|IsPlayerinRange))
  (if _isplayerinrange
    (CallFunction|FacePlayer DeltaSeconds)
    (CallFunction|Move)
    (CallFunction|DamagePlayer)
    (CallFunction|FireProjectile)))

(fn ConstructionScript
  (|CallParentFunction))