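; Health component that gives its owning actor hit points plus a regenerating shield.
; Damage drains the shield first without overflow into health, fires a damage callback, and at zero health triggers the death callback and destroys the owner.
; Each hit stops regeneration and restarts a retriggerable delay.
; Once it expires, Tick restores clamped shield increments, throttled by an interval Delay, firing a regen callback.
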(event Custom|Damage
  (params (Damage%20Amount :type Float%20%28single-precision%29))
  (Variables|Default|SetDamage%20Amount Damage%20Amount)
  (Utilities|FlowControl|Sequence
    (:then_0
      (if (> (Variables|Default|GetShield%20Amount) 0.0)
        (CallFunction|AdjustShieldAmount (* -1 (Variables|Default|GetDamage%20Amount)))
        (Default|CallOnDamageRecieved)
        (else
          (CallFunction|AdjustHealthAmount (* -1 (Variables|Default|GetDamage%20Amount)))
          (Default|CallOnDamageRecieved)
          (if (<= (Variables|Default|GetHP%20Amount) 0.0)
            (CallFunction|Kill)))))
    (:then_1
      (CallFunction|ResetRegen)
      (Variables|Default|SetStart%20Regen false))))

(event Custom|Kill
  (Default|CallOnDeath)
  (Actor|DestroyActor (Components|GetOwner)))

(event Custom|Regen%20Shield%20Delay
  (Utilities|FlowControl|RetriggerableDelay (Variables|Default|GetShield%20Regen%20Delay))
  (Variables|Default|SetStart%20Regen true))

(event Custom|Reset%20Regen
  (Utilities|FlowControl|RetriggerableDelay (Variables|Default|GetShield%20Regen%20Delay))
  (Variables|Default|SetStart%20Regen true))

(event Custom|Regen%20Shield
  (if (Variables|Default|GetStart%20Regen)
    (if (< (Variables|Default|GetShield%20Amount) (Variables|Default|GetShield%20Max))
      (Utilities|FlowControl|Delay (Variables|Default|GetShield%20Regen%20Interval))
      (if (Variables|Default|GetStart%20Regen)
        (CallFunction|AdjustShieldAmount (Variables|Default|GetShield%20Regen%20Rate))
        (Default|CallOnShieldRegen)))))

(event EventBeginPlay
  (CallFunction|RegenShieldDelay))

(event EventTick
  (params (DeltaSeconds :type Float%20%28single-precision%29))
  (CallFunction|RegenShield))

(fn AdjustShieldAmount
  (params (Amount%20to%20Add :type Float%20%28single-precision%29))
  (bind _output_get (Variables|Default|SetShield%20Amount (Math|Float|Clamp(Float) (+ (Variables|Default|GetShield%20Amount) Amount%20to%20Add) 0.0 (Variables|Default|GetShield%20Max))))
  (return _output_get))

(fn AdjustHealthAmount
  (params (Amount%20to%20Add :type Float%20%28single-precision%29))
  (bind _output_get (Variables|Default|SetHP%20Amount (Math|Float|Clamp(Float) (+ (Variables|Default|GetHP%20Amount) Amount%20to%20Add) 0.0 (Variables|Default|GetHP%20Max))))
  (return _output_get))