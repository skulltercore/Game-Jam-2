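; BP_Level_Camera is a level camera actor that takes over the first player's view on BeginPlay and moves between placed BP_Camera_Position points.
; Each tick it targets the first point found within PlayerDistanceToPoint of the player pawn, keeping the last target otherwise, and eases toward its location.
; With FollowPlayer on, the camera component looks directly at the pawn; otherwise the actor eases to the point's Arrow rotation.
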(event Custom|Face%20Player
  (bind _returnvalue (Game|Player|GetPlayerPawn 0))
  (bind _camera (Variables|Default|GetCamera))
  (if (Variables|Default|GetFollowPlayer)
    (Utilities|IsValid _returnvalue
      (:Is%20Valid
        (Transformation|SetWorldRotation _camera (Math|Rotator|FindLookatRotation (Transformation|GetWorldLocation _camera) (Transformation|GetActorLocation _returnvalue)) false false)))))

(event EventBeginPlay
  (Game|Player|SetViewTargetwithBlend (Game|GetPlayerController 0) self 0.5 "VTBlend_Linear" 0.0 false))

(event Collision|EventActorBeginOverlap
  (params (OtherActor :type Actor%20Object%20Reference)))

(event EventTick
  (params (DeltaSeconds :type Float%20%28single-precision%29))
  (CallFunction|FacePlayer)
  (bind _outactors (Actor|GetAllActorsOfClass "/Game/BPs/Camera/BP_Camera_Position.BP_Camera_Position_C"))
  (bind _array_element (Utilities|Array|ForEachLoopwithBreak _outactors :!label _label)
    (:LoopBody
      (if (<= (Transformation|GetDistanceTo _array_element (Game|Player|GetPlayerPawn 0)) (Variables|Default|GetPlayer%20distance%20to%20point))
        (Variables|Default|SetTargetPoint _array_element)
        (goto _label Break)))
    (:Completed
      (Utilities|IsValid (Variables|Default|GetTargetPoint)
        (:Is%20Valid
          (Transformation|SetActorLocation (Math|Interpolation|VInterpTo (Transformation|GetActorLocation) (Transformation|GetActorLocation (Variables|Default|GetTargetPoint)) DeltaSeconds 5.0) false true)
          (if (not (Variables|Default|GetFollowPlayer))
            (Transformation|SetActorRotation (Math|Interpolation|RInterpTo (Transformation|GetActorRotation) (Transformation|GetWorldRotation (Variables|/Game/BPs/Camera/BP_Camera_Position.BP_Camera_Position_C|GetArrow (Variables|Default|GetTargetPoint))) DeltaSeconds 5.0))))))))

(fn ConstructionScript)